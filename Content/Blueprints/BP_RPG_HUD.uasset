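; BP_RPG_HUD puts the player's RPG HUD on screen, with bars for health, stamina, adrenaline and experience points.
; On BeginPlay it creates a WBP_RPG_HUD widget for player controller 0, stores it and adds it to the viewport.
; Four update events each take a new percentage and pass it straight to the matching progress bar in that widget.
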(event EventBeginPlay
  (bind _returnvalue (UserInterface|CreateWidget "/Game/Blueprints/UI/WBP_RPG_HUD.WBP_RPG_HUD_C" (Game|GetPlayerController 0)))
  (bind _output_get (Variables|Default|SetHUD _returnvalue))
  (UserInterface|Viewport|AddtoViewport _output_get 0))

(event EventUpdateExperiencePointsBar
  (params (NewPercentage :type Float%20%28double-precision%29))
  (Progress|SetPercent (Variables|/Game/Blueprints/UI/WBP_RPG_HUD.WBP_RPG_HUD_C|GetExperiencePointsBar (Variables|Default|GetHUD)) NewPercentage))

(event EventUpdateAdrenalineBar
  (params (NewPercentage :type Float%20%28double-precision%29))
  (Progress|SetPercent (Variables|/Game/Blueprints/UI/WBP_RPG_HUD.WBP_RPG_HUD_C|GetAdrenalineBar (Variables|Default|GetHUD)) NewPercentage))

(event EventUpdateStaminaBar
  (params (NewPercentage :type Float%20%28double-precision%29))
  (Progress|SetPercent (Variables|/Game/Blueprints/UI/WBP_RPG_HUD.WBP_RPG_HUD_C|GetStaminaBar (Variables|Default|GetHUD)) NewPercentage))

(event EventUpdateHealthBar
  (params (NewPercentage :type Float%20%28double-precision%29))
  (Progress|SetPercent (Variables|/Game/Blueprints/UI/WBP_RPG_HUD.WBP_RPG_HUD_C|GetHealthBar (Variables|Default|GetHUD)) NewPercentage))

(fn ConstructionScript)